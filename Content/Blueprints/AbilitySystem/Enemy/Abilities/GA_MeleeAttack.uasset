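; Enemy melee attack gameplay ability that turns the avatar toward its combat target and plays a random tagged attack montage.
; On the montage's gameplay event, it finds live players within a small radius of the tagged combat socket and applies damage effects to non-friends.
; A hit fires the MeleeImpact gameplay cue at the socket, tagged with the montage.
; The ability ends after the event or when the montage completes, interrupts or cancels.
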(event Ability|EventActivateAbility
  (bind _returnvalue (Ability|GetAvatarActorfromActorInfo))
  (bind _returnvalue_2 (Ability|GetAvatarActorfromActorInfo))
  (Variables|Default|SetHasHitTarget false)
  (bind _returnvalue_3 (Class|EnemyInterface|GetCombatTarget(Message) _returnvalue_2))
  (bind _ascombat_interface (Utilities|Casting|CastToCombatInterface _returnvalue_2))
  (Class|CombatInterface|UpdateFacingTarget _ascombat_interface (Transformation|GetActorLocation _returnvalue_3))
  (bind _returnvalue_4 (Class|CombatInterface|GetAttackMontages(Message) (Ability|GetAvatarActorfromActorInfo)))
  (bind _output_get (Variables|Default|SetTaggedMontage (Class|MagicianDamageGameplayAbility|GetRandomTaggedMontagefromArray _returnvalue_4)))
  (|PlayMontageandWaitProxy "None" (.montage _output_get) 1.0 "None" true 1.0 0.0
    (:then
      (Ability|Tasks|WaitGameplayEvent (.montagetag _output_get) 0
        (:EventReceived
          (bind _returnvalue_5 (Class|CombatInterface|GetCombatSocketLocation(Message) _returnvalue (.sockettag _output_get)))
          (bind _outoverlappingactors (Class|MagicianAbilitySystemLibrary|GetLivePlayersWithinRadius _returnvalue (Utilities|Array|MakeArray _returnvalue) 45.0 _returnvalue_5))
          (for _array_element _outoverlappingactors
            (if (Class|MagicianAbilitySystemLibrary|IsNotFriend _array_element (Ability|GetAvatarActorfromActorInfo))
              (Class|MagicianAbilitySystemLibrary|ApplyDamageEffect (Class|MagicianDamageGameplayAbility|MakeDamageEffectParamsfromClassDefaults _array_element))
              (Variables|Default|SetHasHitTarget true)))
          (if (Variables|Default|GetHasHitTarget)
            (Class|GameplayAbility|ExecuteGameplayCuewithParams "(TagName=\"GameplayCue.MeleeImpact\")" (Ability|GameplayCue|MakeGameplayCueParameters :AggregatedSourceTags (GameplayTags|MakeGameplayTagContainerfromTag (.montagetag (Variables|Default|GetTaggedMontage))) :Location _returnvalue_5 :EffectCauser (Ability|GetAvatarActorfromActorInfo) :SourceObject _returnvalue_3)))
          (Ability|EndAbility))))
    (:OnCompleted
      (Ability|EndAbility :!label _label))
    (:OnInterrupted
      (goto _label))
    (:OnCancelled
      (goto _label))))