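; BP_FireBall is the Fire Blast projectile, which flies out from its spawn point and returns to ReturnToActor, then explodes.
; On the server, an outgoing timeline lerps it forward to an apex, then a returning timeline lerps it toward the actor's current location.
; Once within ExplodeDistance, it calls OnHit, applies radial damage with upward-angled knockback and death impulse to nearby live players excluding its owner, and destroys itself.
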(event EventStartOutgoingTimeline
  (Networking|SwitchHasAuthority
    (:Authority
      (Variables|Default|SetInitialLocation (Transformation|GetActorLocation))
      (Variables|Default|SetApexLocation (+ (Variables|Default|GetInitialLocation) (* (Transformation|GetActorForwardVector) (Variables|Default|GetTravelDistance))))
      (bind _outgoingtrack (Timeline|OutgoingTimeline Play)
        (:Update
          (Transformation|SetActorLocation (Math|Vector|Lerp(Vector) (Variables|Default|GetInitialLocation) (Variables|Default|GetApexLocation) _outgoingtrack) false false))
        (:Finished
          (bind _returningtrack (Timeline|ReturningTimeline Play)
            (:Update
              (Transformation|SetActorLocation (Math|Vector|Lerp(Vector) (Variables|Default|GetApexLocation) (Transformation|GetActorLocation (Variables|Default|GetReturnToActor)) _returningtrack) false false)
              (if (CallFunction|IsWithinExplodeDistance)
                (Class|MagicianProjectile|OnHit)
                (bind _outoverlappingactors (Class|MagicianAbilitySystemLibrary|GetLivePlayersWithinRadius self (Utilities|Array|MakeArray (Components|GetOwner) self) 3e+02 (Transformation|GetActorLocation)))
                (Variables|Default|SetOverlappingPlayers _outoverlappingactors)
                (Class|MagicianAbilitySystemLibrary|SetIsRadialDamageEffectParam (Variables|Default|GetExplosionDamageParams) true 5e+01 3e+02 (Transformation|GetActorLocation))
                (for _array_element (Variables|Default|GetOverlappingPlayers)
                  (Class|MagicianAbilitySystemLibrary|SetTargetEffectParamsASC (Variables|Default|GetExplosionDamageParams) (Ability|GetAbilitySystemComponent _array_element))
                  (Class|MagicianAbilitySystemLibrary|SetKnockbackDirection (Variables|Default|GetExplosionDamageParams) (Math|Vector|GetForwardVector (Math|Rotator|MakeRotator (.roll (Math|Rotator|MakeRotfromX (- (Transformation|GetActorLocation _array_element) (Transformation|GetActorLocation)))) 45.0 (.yaw (Math|Rotator|MakeRotfromX (- (Transformation|GetActorLocation _array_element) (Transformation|GetActorLocation)))))) 8e+02)
                  (Class|MagicianAbilitySystemLibrary|SetDeathImpulseDirection (Variables|Default|GetExplosionDamageParams) (- (Transformation|GetActorLocation _array_element) (Transformation|GetActorLocation)) 6e+02)
                  (Class|MagicianAbilitySystemLibrary|ApplyDamageEffect (Variables|Default|GetExplosionDamageParams)))
                (Actor|DestroyActor)))))))))

(fn ConstructionScript)

(fn IsWithinExplodeDistance
  (return (<= (Math|Vector|VectorLength (- (Transformation|GetActorLocation) (Transformation|GetActorLocation (Variables|Default|GetReturnToActor)))) (Variables|Default|GetExplodeDistance))))