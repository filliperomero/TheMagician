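; Fire Bolt projectile actor for the fire ability, with a fallback that cleans up bolts that stop making progress.
; Each Tick runs HandleProjectileWithoutTarget, which compares the current location to the previous frame's.
; When the distance moved is at or below MinDistancePerFrame, it plays the impact sound and effect there and destroys itself.
; The threshold is per frame, with no delta-time scaling.
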(event EventBeginPlay)

(event Collision|EventActorBeginOverlap
  (params (OtherActor :type Actor%20Object%20Reference)))

(event EventTick
  (params (DeltaSeconds :type Float%20%28single-precision%29))
  (CallFunction|HandleProjectileWithoutTarget))

(fn ConstructionScript)

(fn HandleProjectileWithoutTarget
  (Variables|Default|SetActorLocationLastFrame (Variables|Default|GetActorLocationThisFrame))
  (Variables|Default|SetActorLocationThisFrame (Transformation|GetActorLocation))
  (if (<= (Math|Vector|VectorLength (- (Variables|Default|GetActorLocationThisFrame) (Variables|Default|GetActorLocationLastFrame))) (Variables|Default|GetMinDistancePerFrame))
    (Audio|SpawnSoundatLocation (Variables|Default|GetImpactSound) (Variables|Default|GetActorLocationThisFrame) "0, 0, 0" 1.0 1.0 0.0 0 0)
    (Niagara|SpawnSystematLocation (Variables|Default|GetImpactEffect) (Variables|Default|GetActorLocationThisFrame))
    (Actor|DestroyActor)))