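; Flame pillar actor that flickers its fire light in an endless, randomly varied pattern.
; On BeginPlay it randomly picks one of two flame intensity timelines, then picks again whenever the playing one finishes.
; Each timeline update feeds its curve value to ScaleFlameIntensity, which multiplies it by BaseIntensity to set the FireLight intensity.
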(event Custom|StartTimeline_01
  (bind _flameintensity (Timeline|FlameIntensityTimeline_01 PlayFromStart)
    (:Update
      (CallFunction|ScaleFlameIntensity _flameintensity))
    (:Finished
      (CallFunction|ChooseTimeline))))

(event Custom|StartTimeline_02
  (bind _flameintensity (Timeline|FlameIntensityTimeline_02 PlayFromStart)
    (:Update
      (CallFunction|ScaleFlameIntensity _flameintensity))
    (:Finished
      (CallFunction|ChooseTimeline))))

(event Custom|ChooseTimeline
  (switch int (Math|Random|RandomIntegerinRange 0 1)
    (:Default
      (CallFunction|StartTimeline01 :!label _label))
    (:0
      (goto _label))
    (:1
      (CallFunction|StartTimeline02))))

(event EventBeginPlay
  (CallFunction|ChooseTimeline))

(fn ConstructionScript)

(fn ScaleFlameIntensity
  (params (Intensity :type Float%20%28double-precision%29))
  (Rendering|Components|Light|SetIntensity (Variables|Default|GetFireLight) (* Intensity (Variables|Default|GetBaseIntensity))))